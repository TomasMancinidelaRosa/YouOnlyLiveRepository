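; BP_Personaje is a player character that walks along the world X axis and jumps, using Enhanced Input.
; BeginPlay adds the IMC_Personaje mapping context to the local player.
; Movement input drives AddMovementInput, then the sign of X acceleration snaps control rotation yaw to face forward or backward.
; The run action only sets a Sprint variable, which has no effect on movement here.
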(event Input|EnhancedActionEvents|EnhancedInputActionIA_MovimientoPersonaje
  (params (ActionValue :type Float%20%28double-precision%29) (ElapsedSeconds :type Float%20%28double-precision%29) (TriggeredSeconds :type Float%20%28double-precision%29) (InputAction :type Input%20Action%20Object%20Reference :default "/Game/Proyecto/Blueprints/Personaje/InputActions/IA_MovimientoPersonaje.IA_MovimientoPersonaje"))
  (bind _returnvalue (Pawn|GetController))
  ;[1 0 0.00845] Caminar
  (if (Variables|Default|GetAction%20Value)
    (Pawn|Input|AddMovementInput (Math|Vector|MakeVector (Variables|Default|GetWorld%20Direction%20X) 0.0 0.0) ActionValue false)
    (else
      (Pawn|Input|AddMovementInput "1.000000,0.000000,0.000000" ActionValue false)))
  (Math|Float|CompareFloat (.x (Pawn|Components|CharacterMovement|GetCurrentAcceleration (Variables|Character|GetCharacterMovement))) 0.0
    (:>
      (Pawn|SetControlRotation _returnvalue (Math|Rotator|MakeRotator 0.0 0.0 0.0)))
    (:<
      (Pawn|SetControlRotation _returnvalue (Math|Rotator|MakeRotator 0.0 0.0 1.8e+02)))))

(event Input|EnhancedActionEvents|EnhancedInputActionIA_SaltarPersonaje
  (params (ActionValue :type Boolean) (ElapsedSeconds :type Float%20%28double-precision%29) (TriggeredSeconds :type Float%20%28double-precision%29) (InputAction :type Input%20Action%20Object%20Reference :default "/Game/Proyecto/Blueprints/Personaje/InputActions/IA_SaltarPersonaje.IA_SaltarPersonaje"))
  (:Started
    (Character|Jump)))

(event Input|EnhancedActionEvents|EnhancedInputActionIA_Correr
  (params (ActionValue :type Boolean) (ElapsedSeconds :type Float%20%28double-precision%29) (TriggeredSeconds :type Float%20%28double-precision%29) (InputAction :type Input%20Action%20Object%20Reference :default "/Game/Proyecto/Blueprints/Personaje/InputActions/IA_Correr.IA_Correr"))
  (Variables|Default|SetSprint 1.2)
  (Variables|Default|SetAction%20Value ActionValue))

(event EventBeginPlay
  (bind _asplayer_controller (Utilities|Casting|CastToPlayerController (Pawn|GetController)))
  (Input|AddMappingContext (PlayerController|LocalPlayerSubsystems|GetEnhancedInputLocalPlayerSubsystem _asplayer_controller) "/Game/Proyecto/Blueprints/Personaje/InputActions/Mapping/IMC_Personaje.IMC_Personaje" 0 "(bIgnoreAllPressedKeysUntilRelease=True,bForceImmediately=False,bNotifyUserSettings=False)"))

(fn ConstructionScript)